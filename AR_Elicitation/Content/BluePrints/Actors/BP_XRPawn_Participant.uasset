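; Magic Leap participant pawn for what appears to be a gesture-referent study, managing controller input and head-following widgets.
; BeginPlay sets up the gesture reader, right controller and three widgets; Tick soft-locks them ahead of the camera via lerp and look-at rotation.
; Trigger fires the referent or unpauses, bumper forwards presses, and the Magic Leap Home button fixes the cube or quits on double-click.
; The Home action toggles pause, swapping widgets by scale.
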(event Custom|SetWidgets
  (bind _widgetpause (Variables|Default|GetWidgetPause))
  (bind _widgetgestures (Variables|Default|GetWidgetGestures))
  (bind _widgetrefferent (Variables|Default|GetWidgetRefferent))
  ;[1 1 1] Set Widgets
  (Utilities|FlowControl|Sequence
    (:then_0
      (bind _returnvalue (UserInterface|CreateWidget "/Game/Menus/W_Gestures_Recognized.W_Gestures_Recognized_C"))
      (UserInterface|SetWidget _widgetgestures _returnvalue)
      (Transformation|SetWorldScale3D _widgetgestures (Math|Conversions|ToVector(Float) (Variables|Widgets|GetWidgetScaleGestures))))
    (:then_1
      (bind _returnvalue_2 (UserInterface|CreateWidget "/Game/Menus/W_Refferent_Banner.W_Refferent_Banner_C"))
      (UserInterface|SetWidget _widgetrefferent _returnvalue_2)
      (Transformation|SetWorldScale3D _widgetrefferent (Math|Conversions|ToVector(Float) (Variables|Widgets|GetWidgetScaleRefferent))))
    (:then_2
      (bind _returnvalue_3 (UserInterface|CreateWidget "/Game/Menus/W_WaitScreen.W_WaitScreen_C"))
      (UserInterface|SetWidget _widgetpause _returnvalue_3)
      (Transformation|SetWorldScale3D _widgetpause "0, 0, 0"))))

(event Custom|WidgetSoftlock
  (params (DeltaSeconds :type Float%20%28single-precision%29))
  (bind _returnvalue (Game|GetPlayerCameraManager 0))
  (bind _returnvalue_2 (Game|GetPlayerCameraManager 0))
  (bind _widgetgestures (Variables|Default|GetWidgetGestures))
  (bind _widgetrefferent (Variables|Default|GetWidgetRefferent))
  (bind _widgetpause (Variables|Default|GetWidgetPause))
  (bind _returnvalue_3 (Transformation|GetWorldLocation _widgetgestures))
  (bind _returnvalue_4 (Camera|GetCameraLocation _returnvalue_2))
  (bind _returnvalue_5 (Camera|GetCameraLocation _returnvalue))
  (bind _returnvalue_6 (Math|Rotator|FindLookatRotation _returnvalue_3 _returnvalue_5))
  ;[0.2921 0.3021 0.299] SoftLockWidgets
  (bind _output_get (Variables|Widgets|SetLocationTarget (+ _returnvalue_5 (* (Transformation|GetActorForwardVector _returnvalue) (Variables|Widgets|GetWidgetDistance)))))
  (bind _output_get_2 (Variables|Widgets|SetLocationCurrent (Math|Vector|Lerp(Vector) (Variables|Widgets|GetLocationCurrent) _output_get (* DeltaSeconds (Variables|Widgets|GetWidgetInterpSpeed)))))
  (Utilities|FlowControl|Sequence
    (:then_0
      (Transformation|SetWorldLocation _widgetgestures _output_get_2 false false)
      (Transformation|SetWorldRotation _widgetgestures _returnvalue_6 false false))
    (:then_1
      (Transformation|SetWorldLocation _widgetrefferent _output_get_2 false false)
      (Transformation|SetWorldRotation _widgetrefferent _returnvalue_6 false false))
    (:then_2
      (bind _output_get_3 (Variables|Widgets|SetLocationTarget (+ _returnvalue_4 (* (Transformation|GetActorForwardVector _returnvalue_2) (Variables|Widgets|GetWidgetDistancePause)))))
      (bind _output_get_4 (Variables|Widgets|SetLocationCurrent (Math|Vector|Lerp(Vector) (Variables|Widgets|GetLocationCurrent) _output_get_3 (* 0.0 (Variables|Widgets|GetWidgetInterpSpeed)))))
      (Transformation|SetWorldLocation _widgetpause _output_get_4 false false)
      (Transformation|SetWorldRotation _widgetpause (Math|Rotator|FindLookatRotation (Transformation|GetWorldLocation (Variables|Default|GetWidgetPause)) _returnvalue_4) false false))))

(event Custom|HapticMed
  ;[1 0.0389 0.1086] Remote Bindings
  (Class|MagicLeapControllerFunctionLibrary|PlayHapticPattern "Right" "Buzz" "Medium"))

(event EventBeginPlay
  (bind _self self)
  (bind _motioncontroller (Variables|Default|GetMotionController _self))
  ;[1 0.07239 0.1022] Begin Play
  (Utilities|FlowControl|Sequence
    (:then_0
      (CallFunction|FPrint "BP_Participant -> New Game Loaded"))
    (:then_1
      (bind _gesturereader (CallFunction|FGetGestureReader))
      (Variables|Gestures|SetGestureReader _gesturereader))
    (:then_2
      (Utilities|IsValid _motioncontroller
        (:Is%20Valid
          (Variables|/Script/HeadMountedDisplay.MotionControllerComponent|SetMotionSource _motioncontroller "Right")
          (CallFunction|FPrint "BP_Participant->controller set"))
        (:Is%20Not%20Valid
          (CallFunction|FPrint "BP_Participant->Failed to get controllert"))))
    (:then_3
      (CallFunction|SetWidgets))))

(event EventTick
  (params (DeltaSeconds :type Float%20%28single-precision%29))
  ;[1 0.03073 0.02078] Event Tick
  (CallFunction|WidgetSoftlock DeltaSeconds))

(event Input|ActionEvents|InputActionTrigger
  (params (Key :type Key%20Structure))
  ;[1 0.0389 0.1086] Remote Bindings
  ;;[1 1 1] Trigger
  (:Pressed
    (if (Variables|Default|GetIsPaused)
      (CallFunction|FPrint "BP_Participant Trigger Pressed Paused No Event")
      (CallFunction|FPause)
      (else
        (CallFunction|FPrint "BP_Participant Trigger Pressed")
        (Default|CallTriggerReferent)))))

(event Input|ActionEvents|InputActionBumper
  (params (Key :type Key%20Structure))
  ;[1 0.0389 0.1086] Remote Bindings
  ;;[1 1 1] Bumper
  (:Pressed
    (CallFunction|FPrint "BP_Participant Bumpeer Pressed ")
    (Default|CallBumperPressed)))

(event Input|ActionEvents|InputActionHome
  (params (Key :type Key%20Structure))
  ;[1 0.0389 0.1086] Remote Bindings
  ;;[1 1 1] Bumper
  (:Pressed
    (CallFunction|FPause)))

(event Input|KeyboardEvents|MotionControllerRightThumbstick
  (params (Key :type Key%20Structure))
  ;[1 0.0389 0.1086] Remote Bindings
  ;;[1 1 1] Unused Thumbstick and Bumper
)

(event Input|KeyboardEvents|MotionControllerRightTrigger
  (params (Key :type Key%20Structure))
  ;[1 0.0389 0.1086] Remote Bindings
  ;;[1 1 1] Trigger
  (:Pressed
    (if (Variables|Default|GetIsPaused)
      (CallFunction|FPrint "BP_Participant Trigger Pressed Paused No Event")
      (CallFunction|FPause)
      (else
        (CallFunction|FPrint "BP_Participant Trigger Pressed")
        (Default|CallTriggerReferent)))))

(event Input|KeyboardEvents|MotionControllerRightShoulder
  (params (Key :type Key%20Structure))
  ;[1 0.0389 0.1086] Remote Bindings
  ;;[1 1 1] Bumper
  (:Pressed
    (CallFunction|FPrint "BP_Participant Bumpeer Pressed ")
    (Default|CallBumperPressed)))

(event Input|KeyboardEvents|MagicLeapRightHomeButton
  (params (Key :type Key%20Structure))
  ;[1 0.0389 0.1086] Remote Bindings
  ;;[1 1 1] Home Button
  (:Pressed
    (Utilities|DetectDoubleClick
      (:Double%20Click
        (CallFunction|FPrint "BP_Participant End Game")
        (Game|QuitGame 0 "Quit" false))
      (:Single%20Click
        (Default|CallFixCube)
        (CallFunction|FPrint "BP_Participant called fix cube")))))

(fn ConstructionScript)

(fn FSpawnShelf
  (bind _returnvalue (Game|SpawnActorfromClass "/Game/BluePrints/BP_Bounds_Visual.BP_Bounds_Visual_C" (Variables|/Game/GameModes/Game_Instance_AR_Affordances.Game_Instance_AR_Affordances_C|GetShelf_Transform (Variables|Default|GetGameInstance)) "Undefined" 0 0))
  (Variables|Default|SetShelf _returnvalue)
  (CallFunction|FPrint " GameInstance -> Shelf Spawned ")
  (return (Variables|Default|GetShelf)))

(fn FSpawnBuildMaterials
  (Default|FSpawnBuildMaterials (Variables|Default|GetGameInstance)))

(fn FPause
  (if (Variables|Default|GetIsPaused)
    (Utilities|FlowControl|Sequence
      (:then_0
        (Transformation|SetWorldScale3D (Variables|Default|GetWidgetRefferent) (Math|Conversions|ToVector(Float) (Variables|Widgets|GetWidgetScaleRefferent))))
      (:then_1
        (Transformation|SetWorldScale3D (Variables|Default|GetWidgetGestures) (Math|Conversions|ToVector(Float) (Variables|Widgets|GetWidgetScaleGestures))))
      (:then_2
        (Transformation|SetWorldScale3D (Variables|Default|GetWidgetPause) "0, 0, 0"))
      (:then_3
        (Variables|Default|SetIsPaused false)))
    (else
      (Utilities|FlowControl|Sequence
        (:then_0
          (Transformation|SetWorldScale3D (Variables|Default|GetWidgetRefferent) "0, 0, 0"))
        (:then_1
          (Transformation|SetWorldScale3D (Variables|Default|GetWidgetGestures) "0, 0, 0"))
        (:then_2
          (Transformation|SetWorldScale3D (Variables|Default|GetWidgetPause) (Math|Conversions|ToVector(Float) (Variables|Widgets|GetWidgetScalePause))))
        (:then_3
          (Variables|Default|SetIsPaused true))))))